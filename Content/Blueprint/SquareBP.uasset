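; Player character for a square platformer hero, with movement on the X axis, jumping, wall jumps and a pause menu.
; In the air, a trace along the forward axis finds a wall to launch away from, else jumps while JumpCurrentCount is below JumpMaxCount.
; Two timelines drive squash-and-stretch scaling on jump and landing.
; BeginPlay sets game-only input; Pause opens the menu widget and pauses the game.
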(event Custom|WallJump
  (bind _returnvalue (Transformation|GetActorForwardVector))
  ;[0.1228 0.9403 1] WallJump
  (bind (_outhit _returnvalue_2) (Collision|LineTraceByChannel (- (Transformation|GetActorLocation) (* _returnvalue (+ (Components|Capsule|GetScaledCapsuleRadius (Variables|Collision|GetCapsuleComponent)) 1.0))) (+ (Transformation|GetActorLocation) (* _returnvalue (+ (Components|Capsule|GetScaledCapsuleRadius (Variables|Collision|GetCapsuleComponent)) 1.0))) "TraceTypeQuery1" true 0 "None"))
  (if _returnvalue_2
    (Character|LaunchCharacter (Math|Vector|MakeVector (* (Math|Float|Sign(Float) (- (.x (Transformation|GetActorLocation)) (.x (.Location (Collision|BreakHitResult _outhit))))) 3e+03) 0.0 (Variables|/Script/Engine.CharacterMovementComponent|GetJumpZVelocity (Variables|Character|GetCharacterMovement))) true true)
    (CallFunction|JumpFX)
    (elif (< (Variables|Default|GetJumpCurrentCount) (Variables|Default|GetJumpMaxCount))
      (Character|Jump)
      (Variables|Default|SetJumpCount (+ (Variables|Default|GetJumpCount) 1))
      (CallFunction|JumpFX))))

(event Custom|JumpFX
  ;[0 1 0.3811] Jump/LandFx
  (bind _squash (Timeline|Timeline_0 PlayFromStart)
    (:Update
      (Transformation|SetActorScale3D (Math|Vector|Lerp(Vector) "1.000000,1.000000,1.000000" "0.125000,1.500000,2.500000" _squash)))))

(event Custom|LandFX
  ;[0 1 0.3811] Jump/LandFx
  (bind _squash (Timeline|Timeline_1 PlayFromStart)
    (:Update
      (Transformation|SetActorScale3D (Math|Vector|Lerp(Vector) "1.000000,1.000000,1.000000" "2.500000,1.500000,0.125000" _squash)))))

(event EventOnLanded
  (params (Hit :type Hit%20Result%20Structure%20%28by%20ref%29))
  ;[0.1911 1 0.1703] Landed
  (Variables|Default|SetJumpCount 0)
  (CallFunction|LandFX))

(event EventBeginPlay
  ;[1 0.06274 0.1922] Turns off mouse as soon as the level starts
  (Input|SetInputModeGameOnly (Game|GetPlayerController 0)))

(event Input|ActionEvents|InputActionPause
  (params (Key :type Key%20Structure))
  ;[0.8634 0 1] Pause Menu function
  (:Pressed
    (if (not (Variables|Default|GetIsScreenShown))
      (bind _returnvalue (UserInterface|CreateWidget "/Game/Blueprint/MainMenu-PauseMenu/PauseMenu.PauseMenu_C"))
      (UserInterface|Viewport|AddtoViewport _returnvalue 0)
      (Input|SetInputModeGameandUI (Game|GetPlayerController 0) _returnvalue "LockAlways" true)
      (Variables|Default|SetIsScreenShown true)
      (Game|SetGamePaused true))))

(event Input|ActionEvents|InputActionJump
  (params (Key :type Key%20Structure))
  ;[0.09969 0.04501 1] Jumping
  (:Pressed
    (if (AI|Components|NavMovement|IsFalling (Variables|Character|GetCharacterMovement))
      (CallFunction|WallJump)
      (else
        (Character|Jump)
        (Variables|Default|SetJumpCount (+ (Variables|Default|GetJumpCount) 1))
        (CallFunction|JumpFX))))
  (:Released
    (Character|StopJumping)))

(event Input|AxisEvents|InputAxisRight
  (params (AxisValue :type Float%20%28single-precision%29))
  ;[1 0.3482 0.0546] Movement Control
  (Pawn|Input|AddMovementInput "1.500000, 0, 0" AxisValue false))

(fn ConstructionScript
  (Variables|/Script/Engine.CharacterMovementComponent|SetJumpZVelocity (Variables|Character|GetCharacterMovement) 7.9e+02)
  (Variables|Default|SetJumpCount 0))