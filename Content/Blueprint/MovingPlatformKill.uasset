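; Moving platform Blueprint that follows a looping or one-shot timeline path and can destroy actors that hit it.
; The construction script stores its placed location, and a timeline started on BeginPlay adds its track offset to that origin without sweeping.
; The Hit event binds the actor-hit delegate at runtime and replays the timeline; once bound, any hit destroys the other actor.
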(event Custom|OnActorHit_Event_0
  (params (SelfActor :type Actor%20Object%20Reference) (OtherActor :type Actor%20Object%20Reference) (NormalImpulse :type Vector) (Hit :type Hit%20Result%20Structure%20%28by%20ref%29))
  (Actor|DestroyActor OtherActor))

(event EventBeginPlay
  (bind _newtrack_0 (Timeline|Timeline_0 Play)
    (:Update
      (Transformation|SetActorLocation (+ (Variables|Default|GetNewVar_0) _newtrack_0) false false))))

(event Collision|EventHit
  (params (MyComp :type Primitive%20Component%20Object%20Reference) (Other :type Actor%20Object%20Reference) (OtherComp :type Primitive%20Component%20Object%20Reference) (bSelfMoved :type Boolean) (HitLocation :type Vector :default "0, 0, 0") (HitNormal :type Vector :default "0, 0, 0") (NormalImpulse :type Vector :default "0, 0, 0") (Hit :type Hit%20Result%20Structure%20%28by%20ref%29))
  (EventDispatchers|AssignOnActorHit (delegate Custom|OnActorHit_Event_0))
  (bind _newtrack_0 (Timeline|Timeline_0 Play)
    (:Update
      (Transformation|SetActorLocation (+ (Variables|Default|GetNewVar_0) _newtrack_0) false false))))

(fn ConstructionScript
  (bind _returnvalue (Transformation|GetActorLocation))
  (Transformation|SetActorLocation _returnvalue false false)
  (Variables|Default|SetNewVar_0 _returnvalue))